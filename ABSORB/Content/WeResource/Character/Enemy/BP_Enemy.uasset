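; BP_Enemy is an enemy character Blueprint that currently only sets up its walk speed.
; On BeginPlay it runs the parent logic, then calls 初始化 (Initialize), which stores a fixed 移动速度 (move speed) and applies it to CharacterMovement's MaxWalkSpeed.
; Tick and overlap events are disabled placeholders, and the construction script only calls its parent.
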(event `self.ReceiveBeginPlay`
  (`parent.ReceiveBeginPlay`)
  (`self.初始化`))

(fn `UserConstructionScript`
  (`parent.UserConstructionScript`))

(fn `初始化`
  (bind _output_get (set `self.移动速度` 300.0))
  (set `CharacterMovementComponent.MaxWalkSpeed` _output_get (`self.CharacterMovement`)))