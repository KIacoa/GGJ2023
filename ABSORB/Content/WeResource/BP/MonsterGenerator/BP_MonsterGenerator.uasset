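; BP_MonsterGenerator is an actor that spawns enemies at placed generator points according to the game manager's alert level.
; On BeginPlay it caches the game instance and the BP_GameManager.
; Its alert-based spawn function scans all BP_MonsterGeneratorPoint actors and spawns a BP_Enemy, tagged with the point's ID, at each point whose alert level equals the manager's current value.
; Nothing in this Blueprint calls that function.
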(event `self.ReceiveBeginPlay`
  (`self.初始化`))

(fn `UserConstructionScript`)

(fn `初始化`
  (bind _asbp_game_instance (cast `/Game/WeResource/BP/Control/BP_GameInstance` (`GameplayStatics.GetGameInstance`)))
  (set `self.As BP Game Instance` _asbp_game_instance)
  (bind _returnvalue (`GameplayStatics.GetActorOfClass` "/Game/WeResource/BP/GameManager/BP_GameManager.BP_GameManager_C"))
  (set `self.游戏管理器` _returnvalue))

(fn `按警戒值生成敌人`
  (bind _outactors (`GameplayStatics.GetAllActorsOfClass` "/Game/WeResource/BP/MonsterGenerator/BP_MonsterGeneratorPoint.BP_MonsterGeneratorPoint_C"))
  (for _array_element _outactors
    (if (== (`/Game/WeResource/BP/MonsterGenerator/BP_MonsterGeneratorPoint.警戒等级` _array_element) (`/Game/WeResource/BP/GameManager/BP_GameManager.警戒值` (`self.游戏管理器`)))
      (bind `_成功` (`self.生成敌人` (`self.K2_GetActorLocation` _array_element) (`/Game/WeResource/BP/MonsterGenerator/BP_MonsterGeneratorPoint.生成点编号` _array_element)))
      (if `_成功`
        _))))

(fn `生成敌人`
  (params (`位置` :type "Vector Structure") (`编号` :type Integer))
  (returns (`成功` :type Boolean))
  (bind _returnvalue (`|SpawnActorFromClass` "/Game/WeResource/Character/Enemy/BP_Enemy.BP_Enemy_C" (`KismetMathLibrary.MakeTransform` `位置`) "AdjustIfPossibleButAlwaysSpawn" "MultiplyWithRoot" null `编号` null))
  (`/Engine/EditorBlueprintResources/StandardMacros.IsValid` _returnvalue
    (:`Is Valid`
      (return true))
    (:`Is Not Valid`
      (return false))))