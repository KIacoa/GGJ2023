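; AC_Interact is an interaction component that gives its owning actor item data and an interaction state.
; On BeginPlay it caches the owner and loads its item info from DT_InteractInfo, using the item name as the row key.
; Two query functions map the four-value interaction state to separate visible and interactable booleans.
; The interact function is a stub, with a switch on interaction type and a cast to BP_Items but no resulting action.
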(event `self.ReceiveBeginPlay`
  (set `self.拥有者` (`self.GetOwner`))
  (`self.获取物品信息`))

(fn `交互`
  (switch `/Game/WeResource/BP/InteractSystem/E_InteractType` (`.交互类型_14_C4A20D9F482142ACAF7D81BACFD5381F` (break `/Game/WeResource/BP/InteractSystem/ST_InteractInfo` (`self.物品信息`)))
    (:`NewEnumerator0`
      (cast `/Game/WeResource/BP/Items/BP_Items` (`self.拥有者`)))))

(fn `是否可交互`
  (returns (`是否可交互` :type Boolean))
  (switch `/Game/WeResource/BP/InteractSystem/E_InteractState` (`self.交互状态`)
    (:`NewEnumerator0`
      (return true))
    (:`NewEnumerator1`
      (return false))
    (:`NewEnumerator2`
      (return true))
    (:`NewEnumerator3`
      (return false))))

(fn `是否可见`
  (returns (`是否可见` :type Boolean))
  (switch `/Game/WeResource/BP/InteractSystem/E_InteractState` (`self.交互状态`)
    (:`NewEnumerator0`
      (return true))
    (:`NewEnumerator1`
      (return true))
    (:`NewEnumerator2`
      (return false))
    (:`NewEnumerator3`
      (return false))))

(fn `获取物品信息`
  (bind _returnvalue (`|GetDataTableRow` "/Game/WeResource/BP/InteractSystem/DT_InteractInfo.DT_InteractInfo" (`self.物品命名`))
    (:`then`
      (set `self.物品信息` _returnvalue))))