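; BP_Items is an item actor whose static mesh is chosen by its item enum.
; After a short delay on BeginPlay, it caches the player pawn as BP_Hero and runs 初始化 (initialize) only if that cast succeeds.
; 初始化 uses the enum name as the DT_Items row name to set the mesh, printing an error if the row is missing.
; No overlap or pickup logic is implemented.
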(event `self.ReceiveBeginPlay`
  (`KismetSystemLibrary.Delay` 0.2)
  (bind _asbp_hero (cast `/Game/WeResource/Character/Hero/BP_Hero` (`GameplayStatics.GetPlayerPawn` 0)))
  (set `self.As BP Hero` _asbp_hero)
  (`self.初始化`))

(fn `UserConstructionScript`)

(fn `初始化`
  (bind _returnvalue (`|GetDataTableRow` "/Game/WeResource/BP/Items/DT_Items.DT_Items" (`KismetStringLibrary.Conv_StringToName` (`|GetEnumeratorNameAsString` (`self.物品枚举`))))
    (:`then`
      (`StaticMeshComponent.SetStaticMesh` (`self.StaticMesh`) (`.物品模型_10_CB035B3844593D748AC45989E0DEA946` (break `/Game/WeResource/BP/Items/ST_Items` _returnvalue))))
    (:`RowNotFound`
      (`KismetSystemLibrary.PrintString` "未找到对应物品"))))