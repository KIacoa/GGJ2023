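; BP_LevelSwitch is a trigger actor that, despite its name, only resets hero and alert state; it loads no level.
; On BeginPlay, after a short delay, it caches BP_GameManager and the player's BP_Hero.
; The first time the hero overlaps its Box, a DoOnce zeroes the hero's 视野等级 (vision level) and the manager's 警戒值 (alert value).
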(event `self.ReceiveBeginPlay`
  (`KismetSystemLibrary.Delay` 0.5)
  (bind _returnvalue (`GameplayStatics.GetActorOfClass` "/Game/WeResource/BP/GameManager/BP_GameManager.BP_GameManager_C"))
  (set `self.游戏管理器` _returnvalue)
  (bind _asbp_hero (cast `/Game/WeResource/Character/Hero/BP_Hero` (`GameplayStatics.GetPlayerPawn` 0)))
  (set `self.As BP Hero` _asbp_hero))

(event `self.Box.OnComponentBeginOverlap`
  (params (OverlappedComponent :type "PrimitiveComponent Object Reference") (OtherActor :type "Actor Object Reference") (OtherComp :type "PrimitiveComponent Object Reference") (OtherBodyIndex :type Integer) (bFromSweep :type Boolean) (SweepResult :type "HitResult Structure (by ref)"))
  (cast `/Game/WeResource/Character/Hero/BP_Hero` OtherActor)
  (`/Engine/EditorBlueprintResources/StandardMacros.DoOnce` false
    (:`Completed`
      (set `/Game/WeResource/Character/Hero/BP_Hero.视野等级` 0 (`self.As BP Hero`))
      (set `/Game/WeResource/BP/GameManager/BP_GameManager.警戒值` 0 (`self.游戏管理器`)))))

(fn `UserConstructionScript`)