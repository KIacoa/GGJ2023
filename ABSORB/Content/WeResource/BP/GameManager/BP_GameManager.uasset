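; Game manager that bootstraps gameplay on ThirdPersonMap and Map_Level1, provides map switching and manages fog of war.
; BeginPlay starts game-instance loading, polls with delays for a PlayerStart and BP_Hero pawn, spawning and possessing one if needed, then initializes the level and completes loading.
; Fog of war applies dynamic M_Sketching materials to mesh actors, mapping view range to their Contrast parameter; the color input is unused.
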(event `生成玩家`
  (bind _returnvalue (`GameplayStatics.GetActorOfClass` "/Script/Engine.PlayerStart"))
  (bind (_returnvalue_location _returnvalue_rotation) (`KismetMathLibrary.BreakTransform` (`self.GetTransform` _returnvalue)))
  (bind _returnvalue_2 (`|SpawnActorFromClass` "/Game/WeResource/Character/Hero/BP_Hero.BP_Hero_C" (`KismetMathLibrary.MakeTransform` _returnvalue_location _returnvalue_rotation) "Undefined" "SelectDefaultAtRuntime" null null))
  (`Controller.Possess` (`GameplayStatics.GetPlayerController` 0) _returnvalue_2))

(event `self.ReceiveBeginPlay`
  (bind _asbp_game_instance (cast `/Game/WeResource/BP/Control/BP_GameInstance` (`GameplayStatics.GetGameInstance`)))
  (set `self.As BP Game Instance` _asbp_game_instance)
  (bind _returnvalue (`GameplayStatics.GetCurrentLevelName` true))
  (if (or (`KismetStringLibrary.EqualEqual_StrStr` _returnvalue "ThirdPersonMap") (`KismetStringLibrary.EqualEqual_StrStr` _returnvalue "Map_Level1"))
    (`/Game/WeResource/BP/Control/BP_GameInstance.初始化Loading` (`self.As BP Game Instance`))
    (`|ExecutionSequence`
      (:`then_0`
        (bind _returnvalue_2 (`GameplayStatics.GetActorOfClass` "/Script/Engine.PlayerStart" :!label _label))
        (`/Engine/EditorBlueprintResources/StandardMacros.IsValid` _returnvalue_2
          (:`Is Valid`
            (bind _asbp_hero (cast `/Game/WeResource/Character/Hero/BP_Hero` (`GameplayStatics.GetPlayerPawn` 0) :!label _label_2)
              (:`then`
                (set `self.As BP Hero` _asbp_hero)
                (bind _returnvalue_3 (`GameplayStatics.GetCurrentLevelName` true))
                (`/Game/WeResource/BP/Control/BP_GameInstance.初始化` (`self.As BP Game Instance`) _returnvalue_3)
                (`/Game/WeResource/BP/WBP/System/Load/WBP_Load.加载完成` (`/Game/WeResource/BP/Control/BP_GameInstance.WBP_Load` (`self.As BP Game Instance`))))
              (:`CastFailed`
                (`self.生成玩家`)
                (`KismetSystemLibrary.Delay` 0.2)
                (goto _label_2))))
          (:`Is Not Valid`
            (`KismetSystemLibrary.Delay` 0.2)
            (goto _label))))
      (:`then_1`
        (`self.战争迷雾初始化`)))))

(event `切换地图`
  (params (LevelName :type Name :default "Map_MainGame"))
  (`GameplayStatics.OpenLevel` LevelName))

(fn `UserConstructionScript`)

(fn `战争迷雾初始化`
  (`|ExecutionSequence`
    (:`then_0`
      (bind _outactors (`GameplayStatics.GetAllActorsOfClass` null))
      (for _array_element _outactors
        (bind _returnvalue (`PrimitiveComponent.CreateDynamicMaterialInstance` (`/Game/WeResource/BP/GameManager/BP_GameManager.StaticMesh` _array_element) 0 "/Game/StylizedMaterials/StaticMeshMaterials/M_Sketching.M_Sketching" "None"))
        (`KismetArrayLibrary.Array_Add` (`self.战争迷雾范围`) _returnvalue)
        (`MaterialInstanceDynamic.SetScalarParameterValue` _returnvalue "Contrast" (`KismetMathLibrary.MapRangeClamped` 0.2 0.0 1.0 1.0 5.0))))))

(fn `设置战争迷雾`
  (params (`视野范围` :type "Float (double-precision)") (`颜色` :type "LinearColor Structure"))
  (`|ExecutionSequence`
    (:`then_0`
      (for _array_element (`self.战争迷雾范围`)
        (`MaterialInstanceDynamic.SetScalarParameterValue` _array_element "Contrast" (`KismetMathLibrary.MapRangeClamped` `视野范围` 0.0 1.0 1.0 5.0))))))